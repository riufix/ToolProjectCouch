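; Beam effect Blueprint that animates several Niagara and beam-end components by stretching them along their Z axis.
; BeginPlay gathers seven components into ListEffects.
; Tick interpolates each one's world Z scale toward a shared target with FInterpTo, keeping X and Y unchanged.
; Interp speed derives from array index for staggered growth; a zero speed, as at the first index, snaps straight to the target.
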(event EventBeginPlay
  (Utilities|Array|Add (Variables|Default|GetListEffects) (Variables|Default|GetNiagara))
  (Utilities|Array|Add (Variables|Default|GetListEffects) (Variables|Default|GetNiagara1))
  (Utilities|Array|Add (Variables|Default|GetListEffects) (Variables|Default|GetBeamEnd3))
  (Utilities|Array|Add (Variables|Default|GetListEffects) (Variables|Default|GetBeamEnd4))
  (Utilities|Array|Add (Variables|Default|GetListEffects) (Variables|Default|GetBeamEnd5))
  (Utilities|Array|Add (Variables|Default|GetListEffects) (Variables|Default|GetBeamEnd8))
  (Utilities|Array|Add (Variables|Default|GetListEffects) (Variables|Default|GetBeamEnd9)))

(event EventTick
  (params (DeltaSeconds :type Float%20%28single-precision%29))
  (for (_array_element _array_index) (Variables|Default|GetListEffects)
    (Transformation|SetWorldScale3D _array_element (Math|Vector|MakeVector (.X (Math|Vector|BreakVector (Transformation|GetWorldScale _array_element))) (.Y (Math|Vector|BreakVector (Transformation|GetWorldScale _array_element))) (Math|Interpolation|FInterpTo (.Z (Math|Vector|BreakVector (Transformation|GetWorldScale _array_element))) 15.0 DeltaSeconds (* (/ _array_index 3) 3.0))))))

(fn ConstructionScript)