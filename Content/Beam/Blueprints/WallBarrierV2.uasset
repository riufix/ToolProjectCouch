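; WallBarrierV2 is a boundary wall actor that plays Wwise impact sounds when hit by objects implementing ProjectileInterface.
; While DelayContact is true, a BP_BeamCharacter hit plays a contact sound and clears that flag for a short retriggerable-delay cooldown.
; Other hits cast to BP_projectile and pick one of three block-destroy sounds by OwnPower, also gated by DelayContact.
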(event EventBeginPlay)

(event Collision|EventActorBeginOverlap
  (params (OtherActor :type Actor%20Object%20Reference)))

(event Collision|EventHit
  (params (MyComp :type Primitive%20Component%20Object%20Reference) (Other :type Actor%20Object%20Reference) (OtherComp :type Primitive%20Component%20Object%20Reference) (bSelfMoved :type Boolean) (HitLocation :type Vector :default "0, 0, 0") (HitNormal :type Vector :default "0, 0, 0") (NormalImpulse :type Vector :default "0, 0, 0") (Hit :type Hit%20Result%20Structure%20%28by%20ref%29))
  (bind _self self)
  (if (Utilities|DoesObjectImplementInterface Other "/Script/project_BEAM.ProjectileInterface")
    (if (Variables|Default|GetDelayContact)
      (Utilities|Casting|CastToBP_BeamCharacter Other
        (:then
          (Variables|Default|SetDelayContact false)
          (Class|AkGameplayStatics|PostEvent "/Game/WwiseAudio/Events/Default_Work_Unit/FOLEY/Contact_Boundaries/Play_MC_ContactBoundary_Plus.Play_MC_ContactBoundary_Plus" self)
          (Utilities|FlowControl|RetriggerableDelay 0.9)
          (Variables|Default|SetDelayContact true))
        (:CastFailed
          (bind _asbp_projectile (Utilities|Casting|CastToBP_projectile Other))
          (switch int (Variables|/Script/project_BEAM.Projectile|GetownPower _asbp_projectile)
            (:1
              (Class|AkGameplayStatics|PostEvent "/Game/WwiseAudio/Events/Default_Work_Unit/SFX/Destruction/Play_SFX_BlockDestroy_Boundary00_Plus.Play_SFX_BlockDestroy_Boundary00_Plus" _self))
            (:2
              (Class|AkGameplayStatics|PostEvent "/Game/WwiseAudio/Events/Default_Work_Unit/SFX/Destruction/Play_SFX_BlockDestroy_Boundary01_Plus.Play_SFX_BlockDestroy_Boundary01_Plus" _self))
            (:3
              (Class|AkGameplayStatics|PostEvent "/Game/WwiseAudio/Events/Default_Work_Unit/SFX/Destruction/Play_SFX_BlockDestroy_Boundary02_Plus.Play_SFX_BlockDestroy_Boundary02_Plus" _self))))))))

(event EventTick
  (params (DeltaSeconds :type Float%20%28single-precision%29)))

(fn ConstructionScript)