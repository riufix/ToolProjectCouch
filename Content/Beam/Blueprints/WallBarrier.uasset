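; WallBarrier is a boundary wall actor that shows a Niagara effect and plays a contact sound when projectiles hit it.
; On BeginPlay, it passes its X, Y and Z values to the Niagara system as particle count parameters.
; Hits from actors implementing ProjectileInterface post a Wwise boundary-contact event, with a boolean gate and short delay throttling repeat sounds.
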(event EventBeginPlay
  (Class|NiagaraComponent|SetVariableInt (Variables|Default|GetNiagara) "XCount" (Variables|Default|GetXValue))
  (Class|NiagaraComponent|SetVariableInt (Variables|Default|GetNiagara) "YCount" (Variables|Default|GetYValue))
  (Class|NiagaraComponent|SetVariableInt (Variables|Default|GetNiagara) "ZCount" (Variables|Default|GetZValue)))

(event Collision|EventHit
  (params (MyComp :type Primitive%20Component%20Object%20Reference) (Other :type Actor%20Object%20Reference) (OtherComp :type Primitive%20Component%20Object%20Reference) (bSelfMoved :type Boolean) (HitLocation :type Vector :default "0, 0, 0") (HitNormal :type Vector :default "0, 0, 0") (NormalImpulse :type Vector :default "0, 0, 0") (Hit :type Hit%20Result%20Structure%20%28by%20ref%29))
  (if (and (Utilities|DoesObjectImplementInterface Other "/Script/project_BEAM.ProjectileInterface") (Variables|Default|GetDelayContact))
    (Variables|Default|SetDelayContact false)
    (Class|AkGameplayStatics|PostEvent "/Game/WwiseAudio/Events/Default_Work_Unit/FOLEY/Contact_Boundaries/Play_MC_ContactBoundary_Plus.Play_MC_ContactBoundary_Plus" self)
    (Utilities|FlowControl|RetriggerableDelay 0.9)
    (Variables|Default|SetDelayContact true)))

(fn ConstructionScript)