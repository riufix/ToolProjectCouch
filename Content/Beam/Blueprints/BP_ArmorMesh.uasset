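; BP_ArmorMesh is an armor mesh actor that scales itself out and destroys itself after being detached.
; On the OnDetach event, if its Condition flag is set, it waits briefly and then caches the mesh's current relative scale.
; A ScaleOut timeline multiplies that cached scale each update, then destroys the actor when finished.
; The Destroyed event clears the Condition flag.
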(event Custom|OnDetach
  (if (Variables|Default|GetCondition)
    (Utilities|FlowControl|Delay 2.5)
    (Variables|Default|SetRelative%20Scale%203D (Variables|/Script/Engine.SceneComponent|GetRelativeScale3D (Variables|Default|GetArmorMesh)))
    (bind _scaleout (Timeline|ScaleOut PlayFromStart)
      (:Update
        (Transformation|SetRelativeScale3D (Variables|Default|GetArmorMesh) (* (Variables|Default|GetRelative%20Scale%203D) _scaleout)))
      (:Finished
        (Actor|DestroyActor)))))

(event EventDestroyed
  (Variables|Default|SetCondition false))

(fn ConstructionScript)