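; Trigger actor that swaps the skins of Beam characters when at least two stand inside it for a set time.
; Overlap events track the players, and Tick runs a timer that, when full, toggles each SkinIndex, saves it to the game instance and reapplies the skin.
; The swap fires once until fewer than two players remain.
; Timer progress is smoothly interpolated into the CenterOffset parameter of a dynamic material on the cube.
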(event EventBeginPlay
  (bind _asbp_beam_game_instance (Utilities|Casting|CastToBP_BeamGameInstance (Game|GetGameInstance)))
  (Variables|Default|SetAs%20BP%20Beam%20Game%20Instance _asbp_beam_game_instance)
  (bind _returnvalue (Rendering|Material|CreateDynamicMaterialInstance (Variables|Default|GetCube) 0 "/Game/Beam/Asset/VFX/Transform/DigitalizeAlt.DigitalizeAlt" "None" :!class /Script/Engine.PrimitiveComponent))
  (Variables|Default|Setmaterial _returnvalue)
  (Rendering|Material|SetScalarParameterValue (Variables|Default|Getmaterial) "CenterOffset" 0.0 :!class /Script/Engine.MaterialInstanceDynamic))

(event Collision|EventActorBeginOverlap
  (params (OtherActor :type Actor%20Object%20Reference))
  (bind _asbp_beam_character (Utilities|Casting|CastToBP_BeamCharacter OtherActor))
  (Utilities|Array|Add (Variables|Default|Getplayers) _asbp_beam_character)
  (Development|PrintString "ADDED"))

(event EventTick
  (params (DeltaSeconds :type Float%20%28single-precision%29))
  (bind _timemax (Variables|Default|GettimeMax))
  (Utilities|ChangeValue DeltaSeconds)
  (if (>= (Utilities|Array|Length (Variables|Default|Getplayers)) 2)
    (if (not (Variables|Default|GetChangedSkin))
      (bind _output_get (Variables|Default|Settimer (+ (Variables|Default|Gettimer) DeltaSeconds)))
      (Variables|Default|Setvalue (/ _output_get _timemax))
      (if (>= _output_get _timemax)
        (Variables|Default|Settimer 0.0)
        ;[0 0 0] Faut att le truc (si 1 -> 0, si 0 -> 1)
        (for _array_element (Variables|Default|Getplayers)
          (Utilities|ChangeSkin _array_element)
          (Default|SetupSkin _array_element (Class|BeamCharacter|IsPhaseTwo _array_element))
          (Variables|Default|SetChangedSkin true)
          (Variables|Default|Setvalue 0.0)))
      (else
        (Variables|Default|Settimer 0.0 :!label _label)
        (Variables|Default|Setvalue 0.0)))
    (else
      (Variables|Default|SetChangedSkin false)
      (goto _label))))

(event Collision|EventActorEndOverlap
  (params (OtherActor :type Actor%20Object%20Reference))
  (bind _asbp_beam_character (Utilities|Casting|CastToBP_BeamCharacter OtherActor))
  (Utilities|Array|RemoveItem (Variables|Default|Getplayers) _asbp_beam_character)
  (Development|PrintString "REMOVED"))

(fn ConstructionScript)