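; Projectile actor whose Niagara look follows one of four power levels, the top one being a beam with camera shake.
; InitParameters sets speed and capsule size from the current projectile parameters.
; Tick destroys it once travel distance exceeds lifeSpan, and stretches the top-level beam from the start position.
; DestructionEffect disables collision and spawns an explosion, then Tick shrinks the beam width until the actor is destroyed.
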(event EventDestructionEffect
  (params (power :type Integer))
  (Collision|SetCollisionProfileName (Variables|Default|GetCapsule) "NoCollision" false :!class /Script/Engine.PrimitiveComponent)
  (Variables|Default|SetisEndBeam true)
  (Niagara|SpawnSystematLocation "/Game/Beam/Asset/VFX/Explosion/ExploUnit.ExploUnit" (Transformation|GetWorldLocation (Variables|Default|GetForwardPosition)) "0, 0, 0" (Math|Conversions|ToVector(Float) (.width (Variables|Default|GetprojectileCurrentParam)))))

(event EventTick
  (params (DeltaSeconds :type Float%20%28single-precision%29))
  (if (> (Math|Vector|Distance(Vector) (Transformation|GetActorLocation) (Variables|Default|GetStartPosition)) (.lifespan (Variables|Default|GetprojectileCurrentParam)))
    (Class|CameraWorldSubsystem|UnShakeCamera (Subsystems|GetCameraWorldSubsystem))
    (Actor|DestroyActor)
    (elif (Variables|Default|GetisEndBeam)
      (Rendering|SetVisibility (Variables|Default|GetNiagara3_1) false true)
      (bind _output_get (Variables|Default|Setwidth (- (Variables|Default|Getwidth) 0.1)))
      (if (< _output_get 0.0)
        (Actor|DestroyActor)
        (Class|CameraWorldSubsystem|UnShakeCamera (Subsystems|GetCameraWorldSubsystem))
        (else
          (Niagara|SetNiagaraVariable(Float) (Variables|Default|GetNiagara3_2) "BeamWidth" (- (Variables|Default|Getwidth) 0.1))
          (Transformation|SetWorldLocation (Variables|Default|GetNiagara3_2) (Variables|Default|GetStartPosition) false false :!label _label)))
      (else
        (Utilities|ShakeNiv3)
        (if (Rendering|IsVisible (Variables|Default|GetNiagara3_1))
          (Niagara|SetNiagaraVariable(Float) (Variables|Default|GetNiagara3_2) "BeamLength" (/ (Math|Vector|Distance(Vector) (Transformation|GetActorLocation) (Variables|Default|GetStartPosition)) 1e+02))
          (goto _label))))))

(event EventInitParameters
  (bind _returnvalue (Class|ProjectileSettings|GetProjectileSettings))
  (bind _capsule (Variables|Default|GetCapsule))
  (bind _projectilecomponent (Variables|Default|GetprojectileComponent))
  (bind _projectilecurrentparam (Variables|Default|GetprojectileCurrentParam))
  (bind _returnvalue_2 (Class|Projectile|GetPower))
  (CallFunction|ChangeNiagara _returnvalue_2)
  (Variables|/Script/Engine.ProjectileMovementComponent|SetMaxSpeed _projectilecomponent (.speed _projectilecurrentparam))
  (Game|Components|ProjectileMovement|SetVelocityinLocalSpace _projectilecomponent (Math|Vector|MakeVector (.speed _projectilecurrentparam) 0.0 0.0))
  (Components|Capsule|SetCapsuleRadius _capsule (* (.width _projectilecurrentparam) 5e+01) true)
  (Components|Capsule|SetCapsuleHalfHeight _capsule (* (.height _projectilecurrentparam) 5e+01) true)
  (Variables|Default|SetStartPosition (Transformation|GetActorLocation))
  (bind _returnvalue_3 (Class|Projectile|GetPower))
  (if (== _returnvalue_3 3)
    (Class|CameraWorldSubsystem|ShakeCamera (Subsystems|GetCameraWorldSubsystem) (Variables|/Script/project_BEAM.ProjectileSettings|GetshakeForce_Tir3 _returnvalue) (Variables|/Script/project_BEAM.ProjectileSettings|GetshakeSpeed_Tir3 _returnvalue))))

(fn ConstructionScript)

(fn ChangeNiagara
  (params (Power :type Integer%20%28by%20ref%29))
  (switch int Power
    (:0
      (Rendering|SetVisibility (Variables|Default|GetNiagara) true false))
    (:1
      (Rendering|SetVisibility (Variables|Default|GetNiagara1) true false))
    (:2
      (Rendering|SetVisibility (Variables|Default|GetNiagara2) true false))
    (:3
      (Rendering|SetVisibility (Variables|Default|GetNiagara3_1) true false)
      (Rendering|SetVisibility (Variables|Default|GetNiagara3_2) true false))))