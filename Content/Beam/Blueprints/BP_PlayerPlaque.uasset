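; BP_PlayerPlaque is a floor or trigger plaque that tracks which BP_BeamCharacters overlap it and assigns Player only when exactly one is present.
; Any other count clears Player and hides the visuals: the Barrier Niagara effect and a percentage fill on Cube1's dynamic material.
; RenderNiagara sets the barrier's XYZ counts and RenderDigital remaps a percentage into the material; neither is called within this Blueprint.
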(event Collision|EventActorBeginOverlap
  (params (OtherActor :type Actor%20Object%20Reference))
  (bind _playerson (Variables|Default|GetplayersOn))
  (bind _asbp_beam_character (Utilities|Casting|CastToBP_BeamCharacter OtherActor))
  (Utilities|Array|Add _playerson _asbp_beam_character)
  (if (not (== (Utilities|Array|Length _playerson) 1))
    (Variables|Default|Setplayer 0)
    (CallFunction|HideNiagara)
    (else
      (Variables|Default|Setplayer (Utilities|Array|Get(acopy) (Variables|Default|GetplayersOn))))))

(event EventBeginPlay
  (bind _returnvalue (Rendering|Material|CreateDynamicMaterialInstance (Variables|Default|GetCube1) 0 "/Game/Beam/Asset/VFX/Transform/Digital.Digital" "None" :!class /Script/Engine.PrimitiveComponent))
  (Variables|Default|Setdigital _returnvalue)
  (CallFunction|HideNiagara))

(event Collision|EventActorEndOverlap
  (params (OtherActor :type Actor%20Object%20Reference))
  (bind _playerson (Variables|Default|GetplayersOn))
  (bind _asbp_beam_character (Utilities|Casting|CastToBP_BeamCharacter OtherActor))
  (for (_array_element _array_index) _playerson
    (if (== _array_element _asbp_beam_character)
      (Utilities|Array|RemoveIndex _playerson _array_index)))
  (if (not (== (Utilities|Array|Length (Variables|Default|GetplayersOn)) 1))
    (Variables|Default|Setplayer 0)
    (CallFunction|HideNiagara)
    (else
      (Variables|Default|Setplayer (Utilities|Array|Get(acopy) (Variables|Default|GetplayersOn))))))

(fn ConstructionScript)

(fn RenderNiagara
  (params (X :type Integer%20%28by%20ref%29) (Y :type Integer%20%28by%20ref%29) (Z :type Integer%20%28by%20ref%29))
  (bind _barrier (Variables|Default|GetBarrier))
  (Class|NiagaraComponent|SetAsset _barrier (Variables|Default|GetniagaraAsset) true)
  (Class|NiagaraComponent|SetVariableInt _barrier "XCount" X)
  (Class|NiagaraComponent|SetVariableInt _barrier "YCount" Y)
  (Class|NiagaraComponent|SetVariableInt _barrier "ZCount" Z))

(fn HideNiagara
  (Class|NiagaraComponent|SetAsset (Variables|Default|GetBarrier) 0 true)
  (Rendering|Material|SetScalarParameterValue (Variables|Default|Getdigital) "Pourcentage" -0.2 :!class /Script/Engine.MaterialInstanceDynamic))

(fn RenderDigital
  (params (percent :type Float%20%28double-precision%29%20%28by%20ref%29))
  (Rendering|Material|SetScalarParameterValue (Variables|Default|Getdigital) "Pourcentage" (/ (- percent 0.3) 1.4) :!class /Script/Engine.MaterialInstanceDynamic))