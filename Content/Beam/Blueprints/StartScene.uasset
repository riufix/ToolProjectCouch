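; StartScene is a per-level setup actor that opens either the wait room or an arena match, switched by IsWaitRoom.
; On BeginPlay it spawns time dilation and end-animation actors, sets Wwise volumes, starts the matching audio and shows the wait room widget if needed.
; It skins each BeamCharacter from the GameInstance, then freezes players during a timed camera shake.
; Music events advance three arena music steps or end them with crowd exclamation.
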(event Custom|OnMusicChange
  (if (not (Variables|Default|GetIsWaitRoom))
    (switch int (Variables|Default|GetMusicStep)
      (:1
        (Variables|Default|SetMusicStep 2)
        (Class|AkGameplayStatics|PostEvent "/Game/WwiseAudio/Events/Default_Work_Unit/MUSIC/Step1/Stop_Music_step_1.Stop_Music_step_1")
        (Class|AkGameplayStatics|PostEvent "/Game/WwiseAudio/Events/Default_Work_Unit/MUSIC/Step2/Play_Music_step_2.Play_Music_step_2"))
      (:2
        (Variables|Default|SetMusicStep 3)
        (Class|AkGameplayStatics|PostEvent "/Game/WwiseAudio/Events/Default_Work_Unit/MUSIC/Step2/Stop_Music_step_2.Stop_Music_step_2")
        (Class|AkGameplayStatics|PostEvent "/Game/WwiseAudio/Events/Default_Work_Unit/MUSIC/Step3/Play_Music_step_3.Play_Music_step_3")))))

(event Custom|OnMusicEnd
  (if (not (Variables|Default|GetIsWaitRoom))
    (Class|AkGameplayStatics|PostEvent "/Game/WwiseAudio/Events/Default_Work_Unit/MUSIC/Step1/Stop_Music_step_1.Stop_Music_step_1")
    (Class|AkGameplayStatics|PostEvent "/Game/WwiseAudio/Events/Default_Work_Unit/MUSIC/Step2/Stop_Music_step_2.Stop_Music_step_2")
    (Class|AkGameplayStatics|PostEvent "/Game/WwiseAudio/Events/Default_Work_Unit/MUSIC/Step3/Stop_Music_step_3.Stop_Music_step_3")
    (Class|AkGameplayStatics|PostEvent "/Game/WwiseAudio/Events/Default_Work_Unit/AMB/Stop_AMB_Arena_Crowd_Loop.Stop_AMB_Arena_Crowd_Loop")
    (Class|AkGameplayStatics|PostEvent "/Game/WwiseAudio/Events/Default_Work_Unit/AMB/Play_AMB_Arena_Exclamation_Plus.Play_AMB_Arena_Exclamation_Plus")))

(event EventBeginPlay
  (bind _returnvalue (Math|Transform|MakeTransform "5000.000000,0.000000,5000.000000"))
  (bind _returnvalue_2 (Subsystems|GetCameraWorldSubsystem))
  (Game|SpawnActorfromClass "/Game/Beam/Blueprints/BP_TimeDilationManager.BP_TimeDilationManager_C" _returnvalue "Undefined" "MultiplyWithRoot" 0 0)
  ;[1 1 1] ADD ANIM END (pour pas à l'ajouter à chaque scene)
  (Game|SpawnActorfromClass "/Game/Beam/Blueprints/AnimEnd.AnimEnd_C" _returnvalue "Undefined" "MultiplyWithRoot" 0 0)
  (Class|AkGameplayStatics|PostEvent "/Game/WwiseAudio/Events/Default_Work_Unit/MUSIC/Menu/Stop_Music_E_Menu.Stop_Music_E_Menu")
  (Class|AkGameplayStatics|PostEvent "/Game/WwiseAudio/Events/Default_Work_Unit/AMB/Stop_AMB_WaitRoom_Loop.Stop_AMB_WaitRoom_Loop")
  ;[1 1 1] Valeur du son
  (Class|AkGameplayStatics|SetRTPCValue "/Game/WwiseAudio/Game_Parameters/Default_Work_Unit/Volume_Music.Volume_Music" 2e+01)
  (Class|AkGameplayStatics|SetRTPCValue "/Game/WwiseAudio/Game_Parameters/Default_Work_Unit/Volume_SFX.Volume_SFX" 2e+01)
  (Class|AkGameplayStatics|SetRTPCValue "/Game/WwiseAudio/Game_Parameters/Default_Work_Unit/Volume_Voices.Volume_Voices" 8e+01)
  (Class|AkGameplayStatics|SetRTPCValue "/Game/WwiseAudio/Game_Parameters/Default_Work_Unit/Volume_Ambiant.Volume_Ambiant" 1e+01)
  (Class|AkGameplayStatics|SetRTPCValue "/Game/WwiseAudio/Game_Parameters/Default_Work_Unit/Volume_Main.Volume_Main" 1e+02)
  (if (Variables|Default|GetIsWaitRoom)
    (Class|AkGameplayStatics|PostEvent "/Game/WwiseAudio/Events/Default_Work_Unit/MUSIC/Menu/Play_Music_E_Menu.Play_Music_E_Menu")
    (Class|AkGameplayStatics|PostEvent "/Game/WwiseAudio/Events/Default_Work_Unit/AMB/Play_AMB_WaitRoom_Loop.Play_AMB_WaitRoom_Loop")
    (bind _returnvalue_3 (UserInterface|CreateWidget "/Game/WaitRoomWidget.WaitRoomWidget_C" (Game|GetPlayerController 0)))
    (UserInterface|Viewport|AddtoViewport _returnvalue_3 0)
    (else
      (Class|AkGameplayStatics|PostEvent "/Game/WwiseAudio/Events/Default_Work_Unit/MUSIC/Step1/Play_Music_step_1.Play_Music_step_1")
      (Class|AkGameplayStatics|PostEvent "/Game/WwiseAudio/Events/Default_Work_Unit/AMB/Play_AMB_Arena_Crowd_Loop.Play_AMB_Arena_Crowd_Loop" 0 0 0 false)
      (Class|AkGameplayStatics|PostEvent "/Game/WwiseAudio/Events/Default_Work_Unit/AMB/Play_AMB_Futuristic_Town_Loop.Play_AMB_Futuristic_Town_Loop" 0 0 0 false)
      (Variables|Default|SetMusicStep 1)))
  (Utilities|FlowControl|DelayUntilNextTick)
  (bind _asmatch_game_mode (Utilities|Casting|CastToMatchGameMode (Game|GetGameMode)))
  (bind _output_get (Variables|Default|SetAsMatchGameMode _asmatch_game_mode))
  (bind _asbp_beam_game_instance (Utilities|Casting|CastToBP_BeamGameInstance (Game|GetGameInstance)))
  (bind _output_get_2 (Variables|Default|SetAs%20BP%20Beam%20Game%20Instance _asbp_beam_game_instance))
  (bind _outactors (Actor|GetAllActorsOfClass "/Game/Beam/Blueprints/BP_BeamCharacter.BP_BeamCharacter_C"))
  (for _array_element _outactors
    (bind _asbp_beam_character (Utilities|Casting|CastToBP_BeamCharacter _array_element))
    (Default|ChangeOutlineColor _asbp_beam_character)
    (bind _returnvalue_4 (Class|GMBeamGameInstance|GetControllertoSkin _output_get_2 (Class|BeamCharacter|GetPlayerIndex _asbp_beam_character)))
    (Variables|/Game/Beam/Blueprints/BP_BeamCharacter.BP_BeamCharacter_C|SetSkinIndex _asbp_beam_character _returnvalue_4)
    (Default|SetupSkin _asbp_beam_character false)
    (Class|BeamCharacter|SetCantDie _asbp_beam_character (Variables|Default|GetIsWaitRoom)))
  (Class|MatchGameMode|FreezePlayers _output_get)
  (Class|CameraWorldSubsystem|ShakeCamera _returnvalue_2 3e+01 2e+01)
  (Utilities|FlowControl|Delay 4.0)
  (Class|MatchGameMode|UnFreezePlayers _output_get)
  (Class|CameraWorldSubsystem|UnShakeCamera _returnvalue_2)
  (if (not (Variables|Default|GetIsWaitRoom))
    (Class|AkGameplayStatics|PostEvent "/Game/WwiseAudio/Events/Default_Work_Unit/SFX/Play_SFX_RoundStart.Play_SFX_RoundStart")
    (Class|AkGameplayStatics|PostEvent "/Game/WwiseAudio/Events/Default_Work_Unit/VOICES/Play_VOC_RoundStart_Plus.Play_VOC_RoundStart_Plus")))

(fn ConstructionScript)