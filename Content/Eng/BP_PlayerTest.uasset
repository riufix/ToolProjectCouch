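; BP_PlayerTest is a test player Blueprint for trying out aim input through Enhanced Input.
; On BeginPlay it casts the first player controller to PC_AimTest and adds the IMC_AimTest mapping context.
; The IA_Aim action passes its value and the actor's location to PlayerAim's AimDir, then prints the resulting direction for debugging.
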(event Input|EnhancedActionEvents|EnhancedInputActionIA_Aim
  (params (ActionValue :type Vector%202D%20Structure) (ElapsedSeconds :type Float%20%28double-precision%29) (TriggeredSeconds :type Float%20%28double-precision%29) (InputAction :type Input%20Action%20Object%20Reference :default "/Game/Eng/IA_Aim.IA_Aim"))
  (bind _returnvalue (Class|PlayerAim|AimDir (Variables|Default|GetPlayerAim) ActionValue (Transformation|GetActorLocation)))
  (Development|PrintString (Utilities|String|ToString(Integer) _returnvalue)))

(event EventBeginPlay
  (bind _aspc_aim_test (Utilities|Casting|CastToPC_AimTest (Game|GetPlayerController 0)))
  (Utilities|IsValid (PlayerController|LocalPlayerSubsystems|GetEnhancedInputLocalPlayerSubsystem _aspc_aim_test)
    (:Is%20Valid
      (Input|AddMappingContext (PlayerController|LocalPlayerSubsystems|GetEnhancedInputLocalPlayerSubsystem _aspc_aim_test) "/Game/Eng/IMC_AimTest.IMC_AimTest" 0 "(bIgnoreAllPressedKeysUntilRelease=True,bForceImmediately=False,bNotifyUserSettings=False)"))))

(fn ConstructionScript)